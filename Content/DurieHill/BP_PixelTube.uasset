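; BP_PixelTube is a DMX pixel tube fixture that broadcasts a single Color to all of its matrix cells.
; BeginPlay enables DMX sending, with the editor affected too.
; Each Tick scales the Color's RGB channels to 0–255 and builds an attribute map with a constant fourth value.
; It then sends every attribute in that map to each cell of the fixture patch's matrix.
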(event EventBeginPlay
  (Class|DMXProtocolBlueprintLibrary|SetSendDMXEnabled true true))

(event Collision|EventActorBeginOverlap
  (params (OtherActor :type Actor%20Object%20Reference)))

(event EventTick
  (params (DeltaSeconds :type Float%20%28single-precision%29))
  (bind _color (Variables|Default|GetColor))
  (bind (_r _g _b) (Math|Color|BreakColor _color))
  (Variables|Default|SetAttributeMap (Utilities|Map|MakeMap "(Name=\"Red\")" (Math|Float|Truncate (* _r 255.0)) "(Name=\"Green\")" (Math|Float|Truncate (* _g 255.0)) "(Name=\"Blue\")" (Math|Float|Truncate (* _b 255.0)) "(Name=\"White\")" 1))
  (bind _output_get (Variables|Default|SetFixturePatch (Class|DMXComponent|GetFixturePatch (Variables|Default|GetDMX))))
  (bind _cells (Class|DMXEntityFixturePatch|GetAllMatrixCells _output_get))
  (for _array_element _cells
    (bind _keys (Utilities|Map|Keys (Variables|Default|GetAttributeMap)))
    (for _array_element_2 _keys
      (Class|DMXEntityFixturePatch|SendMatrixCellValue (Variables|Default|GetFixturePatch) (.coordinate _array_element) _array_element_2 (.Value (Utilities|Map|Find (Variables|Default|GetAttributeMap) _array_element_2))))))

(fn ConstructionScript)